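; Agora media player observer in the MediaPlayer API example that shows or removes the player's video view as its source state changes.
; When opening completes, it makes a video view on the supplied UI canvas panel, using the media player ID as the Uid.
; When playback stops, it releases that view, with both operations updating a stored view map.
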(event `self.OnPlayerSourceStateChanged`
  (params (state :type "EMEDIA_PLAYER_STATE Enum" :default "PLAYER_STATE_IDLE") (ec :type "ENUMWRAP_MEDIA_PLAYER_REASON Structure"))
  (switch `EMEDIA_PLAYER_STATE` state
    (:`PLAYER_STATE_OPEN_COMPLETED`
      (bind _returnvalue (`AgoraBPuMediaPlayer.GetMediaPlayerId` (`AgoraBPuMediaPlayer.GetAgoraMediaPlayer`)))
      (bind _outmap_videoview (`/Game/API-Example/VideoUtilityFunctionLibrary/BFL_VideoManager.MakeVideoView` "VIDEO_SOURCE_MEDIA_PLAYER" "" (`KismetMathLibrary.Conv_IntToInt64` _returnvalue) (`self.UI_CanvasPanel`) (`self.ViewMap`) (`KismetSystemLibrary.GetOuterObject` self)))
      (set `self.ViewMap` _outmap_videoview))
    (:`PLAYER_STATE_STOPPED`
      (bind _returnvalue_2 (`AgoraBPuMediaPlayer.GetMediaPlayerId` (`AgoraBPuMediaPlayer.GetAgoraMediaPlayer`)))
      (bind _outmap_videoview_2 (`/Game/API-Example/VideoUtilityFunctionLibrary/BFL_VideoManager.Release Video View` "VIDEO_SOURCE_MEDIA_PLAYER" "" (`KismetMathLibrary.Conv_IntToInt64` _returnvalue_2) (`self.ViewMap`) (`KismetSystemLibrary.GetOuterObject` self)))
      (set `self.ViewMap` _outmap_videoview_2))))

(fn `SetUICanvasPanel`
  (params (NewParam :type "CanvasPanel Object Reference"))
  (set `self.UI_CanvasPanel` NewParam))