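; Callback executor for the screen-share-while-video-call API example, creating and releasing video views on a UI canvas as users join and leave.
; Local join and leave events match the connection's UID against stored camera and screen-share UIDs to manage a camera view or primary-screen view.
; Remote join and offline events manage per-user remote views, skipping both local UIDs so the user's own streams are not shown as remote.
; Leaving a channel also releases all remote views.
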(event `self.OnJoinChannelSuccess`
  (params (Connection :type "RtcConnection Structure (by ref)") (Elapsed :type Integer))
  (`|ExecutionSequence`
    (:`then_0`
      (if (== Connection_localUid (`self.UID_Camera`))
        (bind _outmap_videoview (`/Game/API-Example/VideoUtilityFunctionLibrary/BFL_VideoManager.MakeVideoView` "VIDEO_SOURCE_CAMERA_PRIMARY" "" 0 (`self.UI_CanvasPanel`) (`self.LocalVideoViewMap`) (`KismetSystemLibrary.GetOuterObject` self)))
        (set `self.LocalVideoViewMap` _outmap_videoview)))
    (:`then_1`
      (if (== Connection_localUid (`self.UID_ScreenShare`))
        (bind _outmap_videoview_2 (`/Game/API-Example/VideoUtilityFunctionLibrary/BFL_VideoManager.MakeVideoView` "VIDEO_SOURCE_SCREEN_PRIMARY" "" 0 (`self.UI_CanvasPanel`) (`self.LocalVideoViewMap`) (`KismetSystemLibrary.GetOuterObject` self)))
        (set `self.LocalVideoViewMap` _outmap_videoview_2)))))

(event `self.OnLeaveChannel`
  (params (connection :type "RtcConnection Structure (by ref)") (stats :type "RtcStats Structure (by ref)"))
  (`|ExecutionSequence`
    (:`then_0`
      (if (== connection_localUid (`self.UID_Camera`))
        (bind _outmap_videoview (`/Game/API-Example/VideoUtilityFunctionLibrary/BFL_VideoManager.Release Video View` "VIDEO_SOURCE_CAMERA_PRIMARY" "" 0 (`self.LocalVideoViewMap`) (`KismetSystemLibrary.GetOuterObject` self)))
        (set `self.LocalVideoViewMap` _outmap_videoview)))
    (:`then_1`
      (if (== connection_localUid (`self.UID_ScreenShare`))
        (bind _outmap_videoview_2 (`/Game/API-Example/VideoUtilityFunctionLibrary/BFL_VideoManager.Release Video View` "VIDEO_SOURCE_SCREEN_PRIMARY" "" 0 (`self.LocalVideoViewMap`) (`KismetSystemLibrary.GetOuterObject` self)))
        (set `self.LocalVideoViewMap` _outmap_videoview_2)))
    (:`then_2`
      (bind _outmap_frameid2videoview (`/Game/API-Example/VideoUtilityFunctionLibrary/BFL_VideoManager.ReleaseAllRemoteVideoView` (`self.RemoteVideoViewMap`) (`KismetSystemLibrary.GetOuterObject` self)))
      (set `self.RemoteVideoViewMap` _outmap_frameid2videoview))))

(event `self.OnUserJoined`
  (params (connection :type "RtcConnection Structure (by ref)") (RemoteUid :type Integer64) (Elapsed :type Integer))
  (bind _ret (`self.IsNotLocalUID` RemoteUid))
  (if _ret
    (bind _outmap_videoview (`/Game/API-Example/VideoUtilityFunctionLibrary/BFL_VideoManager.MakeVideoView` "VIDEO_SOURCE_REMOTE" connection_channelId RemoteUid (`self.UI_CanvasPanel`) (`self.RemoteVideoViewMap`) (`KismetSystemLibrary.GetOuterObject` self)))
    (set `self.RemoteVideoViewMap` _outmap_videoview)))

(event `self.OnUserOffline`
  (params (connection :type "RtcConnection Structure (by ref)") (RemoteUid :type Integer64) (Reason :type "EUSER_OFFLINE_REASON_TYPE Enum" :default "USER_OFFLINE_QUIT"))
  (bind _ret (`self.IsNotLocalUID` RemoteUid))
  (if _ret
    (bind _outmap_videoview (`/Game/API-Example/VideoUtilityFunctionLibrary/BFL_VideoManager.Release Video View` "VIDEO_SOURCE_REMOTE" connection_channelId RemoteUid (`self.RemoteVideoViewMap`) (`KismetSystemLibrary.GetOuterObject` self)))
    (set `self.RemoteVideoViewMap` _outmap_videoview)))

(fn `IsNotLocalUID`
  (params (`Remote UID` :type Integer64))
  (returns (Ret :type Boolean))
  (if (!= `Remote UID` (`self.UID_Camera`))
    (if (!= (`self.UID_ScreenShare`) `Remote UID`)
      (return true)
      (else
        _)))
  (return false))

(fn `SetUIDs`
  (params (UID_Camera :type Integer64) (UID_ScreenShare :type Integer64))
  (set `self.UID_Camera` UID_Camera)
  (set `self.UID_ScreenShare` UID_ScreenShare))