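; Callback executor for the JoinChannelAudio API example, reporting voice channel events as debug text.
; Handles join success, channel leave, and remote user join or offline events, printing each with the user ID where provided.
; The volume indication event prints the total volume, then loops over the speakers to print each one's UID and volume.
; It only prints, changing no state.
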(event `self.OnJoinChannelSuccess`
  (params (Channel :type String) (Uid :type Integer64) (Elapsed :type Integer))
  (`KismetSystemLibrary.PrintString` null "Join Channel Success"))

(event `self.OnLeaveChannel`
  (params (stats :type "RtcStats Structure (by ref)"))
  (`KismetSystemLibrary.PrintString` null "Leave Channel"))

(event `self.OnUserJoined`
  (params (uid :type Integer64) (elapsed :type Integer))
  (`KismetSystemLibrary.PrintString` null (`KismetStringLibrary.Concat_StrStr` "User Joined UId" (`KismetTextLibrary.Conv_TextToString` (`KismetTextLibrary.Conv_Int64ToText` uid)))))

(event `self.OnUserOffline`
  (params (uid :type Integer64) (reason :type "EUSER_OFFLINE_REASON_TYPE Enum" :default "USER_OFFLINE_QUIT"))
  (`KismetSystemLibrary.PrintString` null (`KismetStringLibrary.Concat_StrStr` "User Offline UId" (`KismetTextLibrary.Conv_TextToString` (`KismetTextLibrary.Conv_Int64ToText` uid)))))

(event `self.OnAudioVolumeIndication`
  (params (speakers :type "Array of AudioVolumeInfo Structure (by ref)") (totalVolume :type Integer))
  (`KismetSystemLibrary.PrintString` null (`KismetStringLibrary.Concat_StrStr` "OnAudioVolumeIndication" "Toal Volume" (`KismetStringLibrary.Conv_IntToString` totalVolume)))
  (for _array_element speakers
    (`KismetSystemLibrary.PrintString` null (`KismetStringLibrary.Concat_StrStr` "Uid" (`KismetTextLibrary.Conv_TextToString` (`KismetTextLibrary.Conv_Int64ToText` (break `AudioVolumeInfo` _array_element))) "Volume" (`KismetTextLibrary.Conv_TextToString` (`KismetTextLibrary.Conv_Int64ToText` (`.volume` (break `AudioVolumeInfo` _array_element))))))))