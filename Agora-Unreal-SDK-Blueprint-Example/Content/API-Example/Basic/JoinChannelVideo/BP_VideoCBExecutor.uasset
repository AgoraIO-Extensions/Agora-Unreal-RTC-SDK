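; BP_VideoCBExecutor handles channel callbacks for the JoinChannelVideo API example, creating and releasing on-screen video views.
; Join success and leave events manage the local view, while user joined and offline events manage remote views by Uid.
; Views are auto-sized on a canvas panel supplied through SetUICanvasPanel and tracked in separate local and remote maps.
; The outer object serves as world context for the view helper calls.
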(event `self.OnJoinChannelSuccess`
  (params (Channel :type String) (Uid :type Integer64) (Elapsed :type Integer))
  ;[1 1 1] MakeVideoView: set AudioSize to True, make the View Image auo-sized
  (bind _outmap_videoview (`/Game/API-Example/VideoUtilityFunctionLibrary/BFL_VideoManager.MakeVideoView` "VIDEO_SOURCE_CAMERA_PRIMARY" "" 0 (`self.UI_CanvasPanel`) (`self.LocalVideoViewMap`) true (`KismetSystemLibrary.GetOuterObject` self)))
  (set `self.LocalVideoViewMap` _outmap_videoview))

(event `self.OnLeaveChannel`
  (params (stats :type "UABT_RtcStats Structure (by ref)"))
  (bind _outmap_videoview (`/Game/API-Example/VideoUtilityFunctionLibrary/BFL_VideoManager.Release Video View` "VIDEO_SOURCE_CAMERA_PRIMARY" "" 0 (`self.LocalVideoViewMap`) (`KismetSystemLibrary.GetOuterObject` self)))
  (set `self.LocalVideoViewMap` _outmap_videoview))

(event `self.OnUserJoined`
  (params (uid :type Integer64) (elapsed :type Integer))
  ;[1 1 1] MakeVideoView: set AudioSize to True, make the View Image auo-sized
  (bind _outmap_videoview (`/Game/API-Example/VideoUtilityFunctionLibrary/BFL_VideoManager.MakeVideoView` "VIDEO_SOURCE_REMOTE" "" uid (`self.UI_CanvasPanel`) (`self.RemoteVideoViewMap`) true (`KismetSystemLibrary.GetOuterObject` self)))
  (set `self.RemoteVideoViewMap` _outmap_videoview))

(event `self.OnUserOffline`
  (params (uid :type Integer64) (reason :type "EUABT_USER_OFFLINE_REASON_TYPE Enum" :default "USER_OFFLINE_QUIT"))
  (bind _outmap_videoview (`/Game/API-Example/VideoUtilityFunctionLibrary/BFL_VideoManager.Release Video View` "VIDEO_SOURCE_REMOTE" "" uid (`self.RemoteVideoViewMap`) (`KismetSystemLibrary.GetOuterObject` self)))
  (set `self.RemoteVideoViewMap` _outmap_videoview))

(fn `SetUICanvasPanel`
  (params (UI_CanvasPanel :type "CanvasPanel Object Reference"))
  (set `self.UI_CanvasPanel` UI_CanvasPanel))